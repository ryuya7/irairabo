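; BP_StateManager tracks a course run's elapsed time and outcome in the irairabo game.
; TimerStart and TimerStop drive a Timeline whose update accumulates world delta seconds.
; CourseFailed scores by time survived, while CourseClear scores higher for faster times and updates the current course's info, both writing the score to GI_irairabo.
; Both outcomes then call GameFinished to signal the end of the run.
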(event EventBeginPlay
  (bind _asgi_irairabo (Utilities|Casting|CastToGI_irairabo (Game|GetGameInstance)))
  (Variables|Default|SetGI_irairabo _asgi_irairabo))

(event EventCourseFailed
  (Variables|/Game/GameInstance/GI_irairabo.GI_irairabo_C|SetCurrent_Game_Score (Variables|Default|GetGI_irairabo) (Math|Float|Round (* (Variables|Default|GetTime) 1e+03)))
  (Default|CallGameFinished))

(event EventCourseClear
  (bind _gi_irairabo (Variables|Default|GetGI_irairabo))
  (Variables|/Game/GameInstance/GI_irairabo.GI_irairabo_C|SetCurrent_Game_Score (Variables|Default|GetGI_irairabo) (Math|Float|Round (+ 1e+05 (/ 2e+07 (Variables|Default|GetTime)))))
  (Utilities|Struct|SetmembersinCourseInfo (Utilities|Array|Get(acopy) (Variables|/Game/GameInstance/GI_irairabo.GI_irairabo_C|GetCourse_Infos _gi_irairabo) (Variables|/Game/GameInstance/GI_irairabo.GI_irairabo_C|GetCurrent_Course_Num _gi_irairabo)) true)
  (Default|CallGameFinished))

(event EventTimerStop
  (Timeline|Timer Stop
    (:Update
      (Variables|Default|SetTime (+ (Variables|Default|GetTime) (Utilities|Time|GetWorldDeltaSeconds))))))

(event EventTimerStart
  (Timeline|Timer Play
    (:Update
      (Variables|Default|SetTime (+ (Variables|Default|GetTime) (Utilities|Time|GetWorldDeltaSeconds))))))

(fn ConstructionScript)