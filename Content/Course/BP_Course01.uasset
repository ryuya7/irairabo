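; Timed course actor that reports start, clear and failure to BP_StateManager, found at BeginPlay.
; Collision on the course, field and goal stays off until StartPoint is first overlapped, which starts the timer and destroys that point.
; Reaching the goal clears the course, while touching Course01 or leaving FieldCollider fails it, each stopping the timer through its own DoOnce.
; The construction script tints start green and goal red with dynamic materials.
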(event OnComponentBeginOverlap(Start_Point)
  (params (OverlappedComponent :type Primitive%20Component%20Object%20Reference) (OtherActor :type Actor%20Object%20Reference) (OtherComp :type Primitive%20Component%20Object%20Reference) (OtherBodyIndex :type Integer) (bFromSweep :type Boolean) (SweepResult :type Hit%20Result%20Structure%20%28by%20ref%29))
  (Utilities|FlowControl|DoOnce false
    (:Completed
      (Collision|SetCollisionEnabled (Variables|Default|GetCourse01) "QueryAndPhysics")
      (Collision|SetCollisionEnabled (Variables|Default|GetField_Collider) "QueryAndPhysics")
      (Collision|SetCollisionEnabled (Variables|Default|GetGoal_Point) "QueryAndPhysics")
      (Class|BPIFIrairabo|TimerStart(Message) (Variables|Default|GetBP_StateManager))
      (Components|DestroyComponent (Variables|Default|GetStart_Point)))))

(event OnComponentBeginOverlap(Goal_Point)
  (params (OverlappedComponent :type Primitive%20Component%20Object%20Reference) (OtherActor :type Actor%20Object%20Reference) (OtherComp :type Primitive%20Component%20Object%20Reference) (OtherBodyIndex :type Integer) (bFromSweep :type Boolean) (SweepResult :type Hit%20Result%20Structure%20%28by%20ref%29))
  (bind _bp_statemanager (Variables|Default|GetBP_StateManager))
  (Utilities|FlowControl|DoOnce false
    (:Completed
      (Class|BPIFIrairabo|TimerStop(Message) _bp_statemanager)
      (Class|BPIFIrairabo|CourseClear(Message) _bp_statemanager))))

(event OnComponentEndOverlap(Field_Collider)
  (params (OverlappedComponent :type Primitive%20Component%20Object%20Reference) (OtherActor :type Actor%20Object%20Reference) (OtherComp :type Primitive%20Component%20Object%20Reference) (OtherBodyIndex :type Integer))
  (bind _bp_statemanager (Variables|Default|GetBP_StateManager))
  (Utilities|FlowControl|DoOnce false
    (:Completed
      (Class|BPIFIrairabo|TimerStop(Message) _bp_statemanager)
      (Class|BPIFIrairabo|CourseFailed(Message) _bp_statemanager))))

(event OnComponentBeginOverlap(Course01)
  (params (OverlappedComponent :type Primitive%20Component%20Object%20Reference) (OtherActor :type Actor%20Object%20Reference) (OtherComp :type Primitive%20Component%20Object%20Reference) (OtherBodyIndex :type Integer) (bFromSweep :type Boolean) (SweepResult :type Hit%20Result%20Structure%20%28by%20ref%29))
  (bind _bp_statemanager (Variables|Default|GetBP_StateManager))
  (Utilities|FlowControl|DoOnce false
    (:Completed
      (Class|BPIFIrairabo|TimerStop(Message) _bp_statemanager)
      (Class|BPIFIrairabo|CourseFailed(Message) _bp_statemanager))))

(event EventBeginPlay
  (Collision|SetCollisionEnabled (Variables|Default|GetCourse01) "NoCollision")
  (Collision|SetCollisionEnabled (Variables|Default|GetField_Collider) "NoCollision")
  (Collision|SetCollisionEnabled (Variables|Default|GetGoal_Point) "NoCollision")
  (bind _returnvalue (Actor|GetActorOfClass "/Game/Course/BP_StateManager.BP_StateManager_C"))
  (Variables|Default|SetBP_StateManager _returnvalue))

(fn ConstructionScript
  (bind _returnvalue (Rendering|Material|CreateDynamicMaterialInstance (Variables|Default|GetStart_Point) 0 "/Game/Course/MT_SGPoint.MT_SGPoint" "None" :!class /Script/Engine.PrimitiveComponent))
  (Rendering|Material|SetVectorParameterValue _returnvalue "BaseColor" "(R=0.000000,G=1.000000,B=0.000000,A=1.000000)" :!class /Script/Engine.MaterialInstanceDynamic)
  (bind _returnvalue_2 (Rendering|Material|CreateDynamicMaterialInstance (Variables|Default|GetGoal_Point) 0 "/Game/Course/MT_SGPoint.MT_SGPoint" "None" :!class /Script/Engine.PrimitiveComponent))
  (Rendering|Material|SetVectorParameterValue _returnvalue_2 "BaseColor" "(R=1.000000,G=0.000000,B=0.000000,A=1.000000)" :!class /Script/Engine.MaterialInstanceDynamic))